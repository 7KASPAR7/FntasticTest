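; Player character Blueprint that handles WASD movement through hard-coded key events and a timer instead of Tick.
; Each key press rotates the actor's forward vector by that key's angle, stores it as the movement vector and starts a fast looping timer.
; The timer feeds that vector to AddMovementInput, so direction is fixed at press time.
; Releasing any movement key clears the single timer handle.
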(event Custom|Start%20Movement
  (params (Direction :type Rotator))
  (Variables|Default|SetCurrent%20Movement%20Vector (Math|Vector|RotateVector (* (Transformation|GetActorForwardVector) 3) Direction))
  (bind _returnvalue (Utilities|Time|SetTimerbyEvent (delegate Custom|Movement%20per%20tick) 0.01 true)))

(event Custom|Movement%20per%20tick
  (Pawn|Input|AddMovementInput (Variables|Default|GetCurrent%20Movement%20Vector) 1.0 false))

(event Custom|Stop%20Movement
  (if (Utilities|Time|IsValidTimerHandle (stale Custom|Start%20Movement _returnvalue))
    (Utilities|Time|ClearandInvalidateTimerbyHandle (stale Custom|Start%20Movement _returnvalue))))

(event EventBeginPlay)

(event Collision|EventActorBeginOverlap
  (params (OtherActor :type Actor%20Object%20Reference)))

(event EventTick
  (params (DeltaSeconds :type Float%20%28single-precision%29)))

(event Input|KeyboardEvents|W
  (params (Key :type Key%20Structure :default "None"))
  (:Pressed
    (CallFunction|StartMovement "0, 0, 0"))
  (:Released
    (CallFunction|StopMovement)))

(event Input|KeyboardEvents|S
  (params (Key :type Key%20Structure :default "None"))
  (:Pressed
    (CallFunction|StartMovement "0.000000,180.000000, 0"))
  (:Released
    (CallFunction|StopMovement)))

(event Input|KeyboardEvents|D
  (params (Key :type Key%20Structure :default "None"))
  (:Pressed
    (CallFunction|StartMovement "0.000000,90.000000, 0"))
  (:Released
    (CallFunction|StopMovement)))

(event Input|KeyboardEvents|A
  (params (Key :type Key%20Structure :default "None"))
  (:Pressed
    (CallFunction|StartMovement "0.000000,-90.000000, 0"))
  (:Released
    (CallFunction|StopMovement)))

(fn ConstructionScript)